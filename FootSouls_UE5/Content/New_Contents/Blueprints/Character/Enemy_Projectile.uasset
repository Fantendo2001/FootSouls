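; Enemy shooter that turns to face the Genji player when seen and spawns Bullets from its Arrow, with a prototype deflection check.
; A Fire timeline started at BeginPlay triggers the spawns, independently of sight.
; Each Tick traces along the Arrow; striking a deflecting player's DeflectArea triggers a second trace from the player's camera.
; If that trace hits this enemy, it only prints a deflection message, with debug lines drawn.
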(event OnSeePawn(PawnSensing)
  (params (Pawn :type Pawn%20Object%20Reference))
  (Development|PrintString "see pawn")
  (bind _asgenji_player (Utilities|Casting|CastToGenji_Player Pawn))
  (Utilities|FlowControl|Sequence
    (:then_0
      (Transformation|SetActorRotation (Math|Rotator|FindLookatRotation (Transformation|GetActorLocation) (Transformation|GetActorLocation _asgenji_player))))
    (:then_1
      (Utilities|FlowControl|Delay 0.5))))

(event EventBeginPlay
  (Timeline|Fire Play
    (:NewTrack_0
      (Game|SpawnActorfromClass "/Game/New_Contents/Blueprints/Character/Gun/Bullet.Bullet_C" (Transformation|GetWorldTransform (Variables|Default|GetArrow)) "Undefined" 0 0))))

(event Collision|EventActorBeginOverlap
  (params (OtherActor :type Actor%20Object%20Reference)))

(event EventTick
  (params (DeltaSeconds :type Float%20%28single-precision%29))
  (bind _arrow (Variables|Default|GetArrow))
  (bind _returnvalue (Transformation|GetWorldLocation _arrow))
  (bind (_outhit _returnvalue_2) (Collision|LineTraceByChannel _returnvalue (+ _returnvalue (* (Math|Vector|GetForwardVector _arrow) 8e+03) "") "TraceTypeQuery1" false 0 "ForOneFrame"))
  (if _returnvalue_2
    (bind _asgenji_player (Utilities|Casting|CastToGenji_Player (.HitActor (Collision|BreakHitResult _outhit))))
    (if (== (.HitComponent (Collision|BreakHitResult _outhit)) (Variables|/Game/New_Contents/Blueprints/Character/Genji_Player.Genji_Player_C|GetDeflectArea _asgenji_player))
      (if (Variables|/Game/New_Contents/Blueprints/Character/Genji_Player.Genji_Player_C|GetIs%20Deflecting _asgenji_player)
        (bind (_outhit_2 _returnvalue_3) (Collision|LineTraceByChannel (Transformation|GetWorldLocation (Variables|/Game/New_Contents/Blueprints/Character/Genji_Player.Genji_Player_C|GetFirstPersonCamera _asgenji_player)) (+ (Transformation|GetWorldLocation (Variables|/Game/New_Contents/Blueprints/Character/Genji_Player.Genji_Player_C|GetFirstPersonCamera _asgenji_player)) (* (Math|Vector|GetForwardVector (Variables|/Game/New_Contents/Blueprints/Character/Genji_Player.Genji_Player_C|GetFirstPersonCamera _asgenji_player)) 8e+03)) "TraceTypeQuery1" false (Utilities|Array|MakeArray _asgenji_player) "Persistent"))
        (if _returnvalue_3
          (if (== (.HitActor (Collision|BreakHitResult _outhit_2)) self)
            (Development|PrintString "Deflection Hit")))))))

(fn ConstructionScript)