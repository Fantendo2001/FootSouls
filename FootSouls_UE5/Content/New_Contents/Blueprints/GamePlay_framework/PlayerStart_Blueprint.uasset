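; A PlayerStart Blueprint that acts as a checkpoint for Genji_Player.
; When the player overlaps its Box and the stored Spawn differs from this start's PlayerStartTag, it writes the tag to Spawn, plays a sound, prints an activation message and saves the game.
; A zero-length delay after BeginPlay arms the trigger, so overlaps before that are ignored.
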(event OnComponentBeginOverlap(Box)
  (params (OverlappedComponent :type Primitive%20Component%20Object%20Reference) (OtherActor :type Actor%20Object%20Reference) (OtherComp :type Primitive%20Component%20Object%20Reference) (OtherBodyIndex :type Integer) (bFromSweep :type Boolean) (SweepResult :type Hit%20Result%20Structure%20%28by%20ref%29))
  (bind _playerstarttag (Variables|Default|GetPlayerStartTag))
  (if (Variables|Default|GetStartSave)
    (bind _asgenji_player (Utilities|Casting|CastToGenji_Player OtherActor))
    (if (not (== _playerstarttag (Variables|/Game/New_Contents/Blueprints/Character/Genji_Player.Genji_Player_C|GetSpawn _asgenji_player)))
      (Variables|/Game/New_Contents/Blueprints/Character/Genji_Player.Genji_Player_C|SetSpawn _asgenji_player _playerstarttag)
      (Audio|PlaySound2D "/Game/New_Contents/Audio/Powerup_upgrade_21.Powerup_upgrade_21" 1.5 1.0 0.0 0 0)
      (Development|PrintString "Check Point ACTIVATED!" true true "(R=0.000000,G=1.000000,B=0.241976,A=1.000000)" 3.0)
      (Default|SaveGame _asgenji_player "zyf"))))

(event EventBeginPlay
  (Utilities|FlowControl|Delay 0.0)
  (Variables|Default|SetStartSave true))

(fn ConstructionScript)