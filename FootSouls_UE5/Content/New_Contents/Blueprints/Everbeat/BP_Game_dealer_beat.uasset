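; Beat sphere in the Everbeat rhythm game that travels from its parent dealer past a button position.
; An externally called GameTick runs Move, sliding it along local Y, growing it until DealerDistance, then shrinking it until the dealer removes it.
; Overshooting the threshold marks it failed, decrements any positive GameInstance score and swaps to the fail material.
; IsInside reports whether it sits within the timing window.
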(event Custom|GameTick
  (params (DeltaTime :type Float%20%28double-precision%29))
  (Variables|Default|SetDeltaTime DeltaTime)
  (CallFunction|Move))

(event EventBeginPlay)

(event Collision|EventActorBeginOverlap
  (params (OtherActor :type Actor%20Object%20Reference)))

(event EventTick
  (params (DeltaSeconds :type Float%20%28single-precision%29)))

(fn ConstructionScript)

(fn Move
  ;[1 1 1] Move sphere
  (Transformation|AddLocalOffset (Variables|Default|GetSphere) (Math|Vector|MakeVector 0.0 (* (Variables|Default|GetDeltaTime) (Variables|Default|GetMovementSpeed)) 0.0) false false)
  ;[1 1 1] Scale sphere up until the player button, then scale down until their destruction
  (if (< (.Y (Math|Vector|BreakVector (Variables|/Script/Engine.SceneComponent|GetRelativeLocation (Variables|Default|GetSphere)))) (Variables|Default|GetDealerDistance))
    (Variables|Default|SetSize (+ (Variables|Default|GetSize) (* (Variables|Default|GetDeltaTime) (Variables|Default|GetScaleSpeed))))
    (Transformation|SetRelativeScale3D (Variables|Default|GetSphere) (Math|Vector|MakeVector (Variables|Default|GetSize) (Variables|Default|GetSize) (Variables|Default|GetSize)) :!label _label)
    ;[1 1 1] Change material color when the sphere overtake the dealer button position
    (if (and (not (Variables|Default|GetisFailed)) (> (.Y (Math|Vector|BreakVector (Variables|/Script/Engine.SceneComponent|GetRelativeLocation (Variables|Default|GetSphere)))) (+ (Variables|Default|GetDealerDistance) (Variables|Default|GetDistanceThreshold))))
      (Variables|Default|SetisFailed true)
      (bind _asbp_game_instance (Utilities|Casting|CastToBP_GameInstance (Game|GetGameInstance)))
      (if (> (Variables|/Game/New_Contents/Blueprints/Everbeat/BP_GameInstance.BP_GameInstance_C|GetScore _asbp_game_instance) 0)
        (bind _result (Math|Integer|DecrementInt (Variables|/Game/New_Contents/Blueprints/Everbeat/BP_GameInstance.BP_GameInstance_C|GetScore _asbp_game_instance))
          (:%20%20
            (Default|UpdateScore (Variables|/Game/New_Contents/Blueprints/Everbeat/BP_GameInstance.BP_GameInstance_C|GetBP_Game_ref _asbp_game_instance) _result))))
      (Rendering|Material|SetMaterial (Variables|Default|GetSphere) 0 "/Game/New_Contents/Blueprints/Everbeat/MI_Dealer_Beat_Inst_Fail.MI_Dealer_Beat_Inst_Fail"))
    (elif (> (- (Variables|Default|GetSize) (* (Variables|Default|GetDeltaTime) (Variables|Default|GetScaleSpeed))) 0.0)
      (Variables|Default|SetSize (- (Variables|Default|GetSize) (* (Variables|Default|GetDeltaTime) (Variables|Default|GetScaleSpeed))))
      (goto _label)
      (else
        (Variables|Default|SetSize 0.0)
        (Default|RemoveBeat (Variables|Default|GetParentDealer) self)))))

(fn IsInside
  (bind _sphere (Variables|Default|GetSphere))
  (bind _dealerdistance (Variables|Default|GetDealerDistance))
  (bind _distancethreshold (Variables|Default|GetDistanceThreshold))
  (bind _relativelocation (Variables|/Script/Engine.SceneComponent|GetRelativeLocation _sphere))
  (bind _y (Math|Vector|BreakVector _relativelocation))
  (return (and (< _y (+ _dealerdistance _distancethreshold)) (> _y (- _dealerdistance _distancethreshold)))))