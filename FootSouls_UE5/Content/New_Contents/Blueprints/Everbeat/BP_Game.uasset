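; BP_Game is the controller for a music rhythm game, linking the HUD, audio analyzers and BP_Dealer.
; It loads the first MP3 from the game instance's music folder into a muted Tracker and an audible Player, started together.
; Tick detects low-band beats on the Tracker, skips the opening second after the first beat, then spawns dealer beats on rising edges with a cooldown.
; It also forwards pause, score and beat checks; playback end only prints a placeholder.
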(event Custom|OnPlaybackFinished
  ;[1 1 1] To do something of playback end
  (Variables|Default|SetFirstDelayTriggered false)
  (Variables|Default|SetFirstDelay 1.0)
  (Development|PrintString "Show score dialog"))

(event Custom|StartAudioPlayback
  (bind _tracker (Variables|Default|GetTracker))
  ;[1 1 1] Called from the coundown widget when reach zero
  (Class|AudioAnalyzerManager|SetPlaybackVolume _tracker 0.0)
  (Class|AudioAnalyzerManager|PlayEx _tracker 99999 0.0)
  (Variables|Default|SetisPaused false)
  (Class|AudioAnalyzerManager|PlayEx (Variables|Default|GetPlayer) 99999 0.0))

(event Custom|Bonus%20Music)

(event EventBeginPlay
  (bind _asbp_game_instance (Utilities|Casting|CastToBP_GameInstance (Game|GetGameInstance)))
  (Variables|/Game/New_Contents/Blueprints/Everbeat/BP_GameInstance.BP_GameInstance_C|SetBP_Game_ref _asbp_game_instance self)
  ;[1 1 1] User Interface initialization
  (bind _returnvalue (Game|ConstructObjectfromClass self "/Game/New_Contents/Blueprints/UI/Hud.Hud_C"))
  (bind _output_get (Variables|Default|SetHud _returnvalue))
  (Default|ShowUI _output_get)
  ;[1 1 1] To do something of playback end
  (EventDispatchers|BindEventtoOnPlaybackFinished (Variables|Default|GetPlayer) (delegate Custom|OnPlaybackFinished)))

(event EventTick
  (params (DeltaSeconds :type Float%20%28single-precision%29))
  (Variables|Default|SetCooldown (- (Variables|Default|GetCooldown) DeltaSeconds))
  (if (not (Variables|Default|GetisPaused))
    (Variables|Default|SetDeltaTime DeltaSeconds)
    (CallFunction|DealersTick)
    (bind _beats (Class|AudioAnalyzerManager|GetBeatTrackingWLimits (Variables|Default|GetTracker)))
    ;[1 1 1] Discard the first seconds of the analysis
    (if (< (Variables|Default|GetFirstDelay) 0.0)
      (CallFunction|UpdateBeatonSet (and (<= (Variables|Default|GetCooldown) 0.0) (Utilities|Array|Get(acopy) _beats)))
      (elif (Variables|Default|GetFirstDelayTriggered)
        (Variables|Default|SetFirstDelay (- (Variables|Default|GetFirstDelay) (Variables|Default|GetDeltaTime)))
        (elif (Utilities|Array|Get(acopy) _beats)
          (Variables|Default|SetFirstDelayTriggered true))))))

(fn ConstructionScript)

(fn UpdateScore
  (params (New :type Integer))
  (Default|UpdateScore (Variables|Default|GetHud) New))

(fn InitializeAudioManagers
  ;[1 1 1] Construct AudioAnalyzerManager instances in the Game Instance
  (bind _asbp_game_instance (Utilities|Casting|CastToBP_GameInstance (Game|GetGameInstance)))
  (Default|InitializeGame _asbp_game_instance)
  ;[1 1 1] Take the first audio file of the RawMusic
  (bind _asbp_game_instance_2 (Utilities|Casting|CastToBP_GameInstance (Game|GetGameInstance)))
  (bind (_filenames _returnvalue) (Class|AudioAnalyzerManager|GetFolderFiles (Variables|/Game/New_Contents/Blueprints/Everbeat/BP_GameInstance.BP_GameInstance_C|GetBP_AAManager_Player _asbp_game_instance_2) (Utilities|String|Append (Class|KismetSystemLibrary|GetProjectContentDirectory) (Variables|/Game/New_Contents/Blueprints/Everbeat/BP_GameInstance.BP_GameInstance_C|GetRawMusicFolderName _asbp_game_instance_2)) "mp3"))
  (if _returnvalue
    ;[1 1 1] Construct audio file path
    (bind _asbp_game_instance_3 (Utilities|Casting|CastToBP_GameInstance (Game|GetGameInstance)))
    (Variables|/Game/New_Contents/Blueprints/Everbeat/BP_GameInstance.BP_GameInstance_C|SetSongTitle _asbp_game_instance_3 (Utilities|Array|Get(acopy) _filenames))
    (Variables|/Game/New_Contents/Blueprints/Everbeat/BP_GameInstance.BP_GameInstance_C|SetSongPath _asbp_game_instance_3 (Utilities|String|Append (Class|KismetSystemLibrary|GetProjectContentDirectory) (Variables|/Game/New_Contents/Blueprints/Everbeat/BP_GameInstance.BP_GameInstance_C|GetRawMusicFolderName _asbp_game_instance_3) "/" (Utilities|Array|Get(acopy) _filenames)))
    ;[1 1 1] Intializer dealer actor class
    (bind _asbp_dealer (Utilities|Casting|CastToBP_Dealer (Variables|/Script/Engine.ChildActorComponent|GetChildActor (Variables|Default|Getdealer))))
    (Default|InitializeDealer _asbp_dealer (Variables|Default|GetPLAYER_DELAY))
    ;[1 1 1] Initializes Player and Tracker and Beat Tracking analyzer
    (bind _asbp_game_instance_4 (Utilities|Casting|CastToBP_GameInstance (Game|GetGameInstance)))
    (Variables|Default|SetTracker (Variables|/Game/New_Contents/Blueprints/Everbeat/BP_GameInstance.BP_GameInstance_C|GetBP_AAManager_Player _asbp_game_instance_4))
    (Variables|Default|SetPlayer (Variables|/Game/New_Contents/Blueprints/Everbeat/BP_GameInstance.BP_GameInstance_C|GetBP_AAManager_Tracker _asbp_game_instance_4))
    (bind _returnvalue_2 (Class|AudioAnalyzerManager|InitPlayerAudio (Variables|Default|GetTracker) (Variables|/Game/New_Contents/Blueprints/Everbeat/BP_GameInstance.BP_GameInstance_C|GetSongPath _asbp_game_instance_4)))
    (if _returnvalue_2
      (bind _returnvalue_3 (Class|AudioAnalyzerManager|InitPlayerAudio (Variables|Default|GetPlayer) (Variables|/Game/New_Contents/Blueprints/Everbeat/BP_GameInstance.BP_GameInstance_C|GetSongPath _asbp_game_instance_4)))
      (if _returnvalue_3
        _
        (else
          (Development|PrintString "Init Player error")))
      (Class|AudioAnalyzerManager|InitBeatTrackingConfigWLimits (Variables|Default|GetTracker) "All_in_one" 0 (Utilities|Array|MakeArray "(X=0.000000,Y=100.000000)") 0.02 30 false 100 2.6)
      (else
        (Development|PrintString "Init Tracker error")))))

(fn SetPause
  (params (Pause :type Boolean))
  (bind _output_get (Variables|Default|SetisPaused Pause))
  (Class|AudioAnalyzerManager|SetPaused (Variables|Default|GetPlayer) _output_get))

(fn UpdateBeatonSet
  (params (NewBeatState :type Boolean))
  (if (and NewBeatState (not (Variables|Default|GetLastBeatOnSet)))
    (Variables|Default|SetLastBeatOnSet true)
    (Variables|Default|SetCooldown 0.8)
    (CallFunction|SpawnNewBeat)
    (elif (and (not NewBeatState) (Variables|Default|GetLastBeatOnSet))
      (Variables|Default|SetLastBeatOnSet false))))

(fn SpawnNewBeat
  (bind _asbp_dealer (Utilities|Casting|CastToBP_Dealer (Variables|/Script/Engine.ChildActorComponent|GetChildActor (Variables|Default|Getdealer))))
  (Default|SpawnNewBeat _asbp_dealer))

(fn DealersTick
  (bind _asbp_dealer (Utilities|Casting|CastToBP_Dealer (Variables|/Script/Engine.ChildActorComponent|GetChildActor (Variables|Default|Getdealer))))
  (Default|GameTick _asbp_dealer (Variables|Default|GetDeltaTime)))

(fn GameCheckBeat
  (bind _asbp_dealer (Utilities|Casting|CastToBP_Dealer (Variables|/Script/Engine.ChildActorComponent|GetChildActor (Variables|Default|Getdealer))))
  (Default|CheckBeats _asbp_dealer))